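; Enemy actor that damages the player on contact and awards score when shot by a projectile.
; Overlap with the player plays a world camera shake, lowers Health by one, and on reaching zero flags the player dead and shows restart.
; Overlap with a projectile destroys the projectile and increments the first player pawn's Score.
; Either case destroys the enemy, which has no movement or tick logic in this graph.
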(event `self.ReceiveActorBeginOverlap`
  (params (OtherActor :type "Actor Object Reference"))
  (bind _asbp_player (cast `/Game/InfiniteMatrix/Blueprints/BP_Player` OtherActor)
    (:`then`
      (`self.Process Enemy Hit` _asbp_player))
    (:`CastFailed`
      (bind _asprojectile (cast `/Game/InfiniteMatrix/Blueprints/Projectile` OtherActor))
      (`self.K2_DestroyActor` _asprojectile)
      (bind _asbp_player_2 (cast `/Game/InfiniteMatrix/Blueprints/BP_Player` (`GameplayStatics.GetPlayerPawn` 0)))
      (set `/Game/InfiniteMatrix/Blueprints/BP_Player.Score` (+ (`/Game/InfiniteMatrix/Blueprints/BP_Player.Score` _asbp_player_2) 1) _asbp_player_2)))
  (`self.K2_DestroyActor`))

(fn `Process Enemy Hit`
  (params (`Bp player` :type "/Game/InfiniteMatrix/Blueprints/BP_Player Object Reference"))
  (`GameplayStatics.PlayWorldCameraShake` "/Game/InfiniteMatrix/Blueprints/BP_camshake.BP_camshake_C" (`self.K2_GetActorLocation` `Bp player`) 0.0 1000.0)
  (bind _output_get (set `/Game/InfiniteMatrix/Blueprints/BP_Player.Health` (- (`/Game/InfiniteMatrix/Blueprints/BP_Player.Health` `Bp player`) 1) `Bp player`))
  (if (<= _output_get 0)
    (set `/Game/InfiniteMatrix/Blueprints/BP_Player.IsDead` true `Bp player`)
    (`/Game/InfiniteMatrix/Blueprints/BP_Player.DisplayRestart` `Bp player`)))

(fn `UserConstructionScript`)